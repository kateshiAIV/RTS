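; Base enemy character that the player's units can target, attack or stealth-kill.
; It swaps weapon meshes between holster slots and hands, plays per-weapon attack montages, and fires wield, sheath and attack-end callbacks.
; Clicking it assigns it to selected units, hovering shows a decal, and a collision box marks it as a stealth target.
; It exposes patrol, range and speed functions, tracks weapon hand sockets on Tick, and ragdolls with AI logic stopped on death.
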(event OnClicked(CapsuleComponent)
  (params (TouchedComponent :type Primitive%20Component%20Object%20Reference) (ButtonPressed :type Key%20Structure))
  (bind _outactors (Actor|GetAllActorsOfClass "/Game/Core/Character/BP_ParentUnitClass.BP_ParentUnitClass_C"))
  (for _array_element _outactors
    (if (Variables|/Game/Core/Character/BP_ParentUnitClass.BP_ParentUnitClass_C|GetUnitIsSelected _array_element)
      (Default|SetAttackTarget _array_element self))))

(event OnComponentBeginOverlap(StealthKillBoxCollision)
  (params (OverlappedComponent :type Primitive%20Component%20Object%20Reference) (OtherActor :type Actor%20Object%20Reference) (OtherComp :type Primitive%20Component%20Object%20Reference) (OtherBodyIndex :type Integer) (bFromSweep :type Boolean) (SweepResult :type Hit%20Result%20Structure%20%28by%20ref%29))
  (if (not (Variables|Health|GetIsDead))
    (bind _asbp_parent_unit_class (Utilities|Casting|CastToBP_ParentUnitClass OtherActor))
    (Variables|/Game/Core/Character/BP_ParentUnitClass.BP_ParentUnitClass_C|SetCurrentPotentialStealthTarget _asbp_parent_unit_class self)
    (Variables|Stealth|SetStealthBackTrigger true)))

(event OnComponentEndOverlap(StealthKillBoxCollision)
  (params (OverlappedComponent :type Primitive%20Component%20Object%20Reference) (OtherActor :type Actor%20Object%20Reference) (OtherComp :type Primitive%20Component%20Object%20Reference) (OtherBodyIndex :type Integer))
  (if (not (Variables|Health|GetIsDead))
    (bind _asbp_parent_unit_class (Utilities|Casting|CastToBP_ParentUnitClass OtherActor))
    (Variables|/Game/Core/Character/BP_ParentUnitClass.BP_ParentUnitClass_C|SetCurrentPotentialStealthTarget _asbp_parent_unit_class 0)
    (Variables|Stealth|SetStealthBackTrigger false)))

(event OnBeginCursorOver(CapsuleComponent)
  (params (TouchedComponent :type Primitive%20Component%20Object%20Reference))
  (CallFunction|HighlightUnit))

(event OnEndCursorOver(CapsuleComponent)
  (params (TouchedComponent :type Primitive%20Component%20Object%20Reference))
  (CallFunction|UnhighlightUnit))

(event Custom|WieldSword
  (switch Utilities|FlowControl|Switch|SwitchonE_WeaponTypes (Variables|Default|GetCurrentWeapon)
    (:NewEnumerator0
      (Rendering|SetVisibility (Variables|Default|GetWieldedWeapon) true false)
      (Components|SkeletalMesh|SetSkeletalMeshAsset (Variables|Default|GetWeaponSlot1) 0)
      (Variables|Default|SetIsWielding2HandedWeapon true))
    (:NewEnumerator1
      (Components|SkeletalMesh|SetSkeletalMeshAsset (Variables|Default|GetWeaponSlot2) 0)
      (Components|SkeletalMesh|SetSkeletalMeshAsset (Variables|Default|GetSmallWeaponSlot) 0)
      (Components|SkeletalMesh|SetSkeletalMeshAsset (Variables|Default|GetRightHand) "/Game/KoreanTraditionalMartialArts/Meshs/Weapons/Meshs/SKM_SsanggeomR.SKM_SsanggeomR")
      (Components|SkeletalMesh|SetSkeletalMeshAsset (Variables|Default|GetShieldSlot) "/Game/KoreanTraditionalMartialArts/Meshs/Weapons/Meshs/SKM_Deungpae.SKM_Deungpae"))
    (:NewEnumerator9
      (Rendering|SetVisibility (Variables|Default|GetWieldedWeapon) true false)
      (Components|SkeletalMesh|SetSkeletalMeshAsset (Variables|Default|GetWeaponSlot1) 0)
      (Variables|Default|SetIsWielding2HandedWeapon true)))
  (Variables|Default|SetIsWieldingWeapon true)
  (Default|CallOnWieldWeaponEnd))

(event Custom|AttackPlayerPawn
  (Variables|Default|SetbIsPlayingAttackAnimation true)
  (switch Utilities|FlowControl|Switch|SwitchonE_WeaponTypes (Variables|Default|GetCurrentWeapon)
    (:NewEnumerator0
      (Animation|Montage|PlayMontage (Variables|Default|GetWieldedWeapon) "/Game/KoreanTraditionalMartialArts/Animations/Dangpa/Anim_Dangpa_Attack1_Weapon_Montage.Anim_Dangpa_Attack1_Weapon_Montage"
        (:then
          (Animation|Montage|PlayMontage (Variables|Character|GetMesh) "/Game/KoreanTraditionalMartialArts/MannyAnims/M_Anim_Dangpa_Attack1_Soldier_Montage.M_Anim_Dangpa_Attack1_Soldier_Montage"
            (:OnCompleted
              _)
            (:OnInterrupted
              _)))))
    (:NewEnumerator1
      (Animation|Montage|PlayMontage (Variables|Character|GetMesh) "/Game/KoreanTraditionalMartialArts/MannyAnims/M_Anim_Deoungpae_Attack1_Soldier_Montage.M_Anim_Deoungpae_Attack1_Soldier_Montage"
        (:OnCompleted
          _)
        (:OnInterrupted
          _)))
    (:NewEnumerator9
      (Animation|Montage|PlayMontage (Variables|Default|GetWieldedWeapon) "/Game/KoreanTraditionalMartialArts/Animations/Ssangsudo/M_Anim_Ssangsudo_Attack1_Weapon.M_Anim_Ssangsudo_Attack1_Weapon"
        (:then
          (Animation|Montage|PlayMontage (Variables|Character|GetMesh) "/Game/KoreanTraditionalMartialArts/MannyAnims/M_Anim_Ssangsudo_Attack1_Soldier_Montage.M_Anim_Ssangsudo_Attack1_Soldier_Montage"
            (:OnCompleted
              _)
            (:OnInterrupted
              _))))))
  (Variables|Default|SetbIsPlayingAttackAnimation false)
  (Default|CallOnAttackEnd))

(event Custom|Die
  (bind _mesh (Variables|Character|GetMesh))
  (Physics|SetSimulatePhysics _mesh true)
  (Collision|SetCollisionEnabled _mesh "QueryAndPhysics")
  (AI|Logic|StopLogic (Variables|/Script/AIModule.AIController|GetBrainComponent (Variables|Default|GetAs%20AIC%20Enemy%20Base)) ""))

(event Custom|SheathWeapon
  (switch Utilities|FlowControl|Switch|SwitchonE_WeaponTypes (Variables|Default|GetCurrentWeapon)
    (:NewEnumerator0
      (Components|SkeletalMesh|SetSkeletalMeshAsset (Variables|Default|GetWieldedWeapon) "/Game/KoreanTraditionalMartialArts/Meshs/Weapons/Meshs/SKM_Dangpa.SKM_Dangpa")
      (Class|SkeletalMeshComponent|SetAnimClass (Variables|Default|GetWieldedWeapon) "/Game/Core/CharactersNotPlayable/ABP_DangpaWeapon.ABP_DangpaWeapon_C")
      (Rendering|SetVisibility (Variables|Default|GetWieldedWeapon) false false)
      (Components|SkeletalMesh|SetSkeletalMeshAsset (Variables|Default|GetWeaponSlot1) "/Game/KoreanTraditionalMartialArts/Meshs/Weapons/Meshs/SKM_Dangpa.SKM_Dangpa"))
    (:NewEnumerator1
      (Components|SkeletalMesh|SetSkeletalMeshAsset (Variables|Default|GetWieldedWeapon) 0)
      (Class|SkeletalMeshComponent|SetAnimClass (Variables|Default|GetWieldedWeapon))
      (Rendering|SetVisibility (Variables|Default|GetWieldedWeapon) false false)
      (Components|SkeletalMesh|SetSkeletalMeshAsset (Variables|Default|GetWeaponSlot2) "/Game/KoreanTraditionalMartialArts/Meshs/Weapons/Meshs/SKM_Deungpae.SKM_Deungpae")
      (Components|SkeletalMesh|SetSkeletalMeshAsset (Variables|Default|GetSmallWeaponSlot) "/Game/KoreanTraditionalMartialArts/Meshs/Weapons/Meshs/SKM_SsanggeomR.SKM_SsanggeomR"))
    (:NewEnumerator9
      (Components|SkeletalMesh|SetSkeletalMeshAsset (Variables|Default|GetWieldedWeapon) "/Game/KoreanTraditionalMartialArts/Meshs/Weapons/Meshs/SKM_Ssangsudo.SKM_Ssangsudo")
      (Class|SkeletalMeshComponent|SetAnimClass (Variables|Default|GetWieldedWeapon) "/Game/Core/CharactersNotPlayable/ABP_SsangsudoWeapon.ABP_SsangsudoWeapon_C")
      (Rendering|SetVisibility (Variables|Default|GetWieldedWeapon) false false)
      (Components|SkeletalMesh|SetSkeletalMeshAsset (Variables|Default|GetWeaponSlot1) "/Game/KoreanTraditionalMartialArts/Meshs/Weapons/Meshs/SKM_Ssangsudo.SKM_Ssangsudo")))
  (Variables|Default|SetIsWieldingWeapon false)
  (Default|CallOnSheathWeaponEnd))

(event Custom|UnhighlightUnit
  ;[1 1 1] Unhighlight Unit on mouse overlap end
  (Rendering|SetVisibility (Variables|Default|GetDecal) false false))

(event Custom|HighlightUnit
  ;[1 1 1] Highlight Unit on Mouse overlap
  (Rendering|SetVisibility (Variables|Default|GetDecal) true false))

(event EventBeginPlay
  (bind _asaic_enemy_base (Utilities|Casting|CastToAIC_EnemyBase (AI|GetAIController self)))
  (Variables|Default|SetAs%20AIC%20Enemy%20Base _asaic_enemy_base)
  (CallFunction|SheathWeapon))

(event EventTick
  (params (DeltaSeconds :type Float%20%28single-precision%29))
  (Variables|Default|SetLeftHandPose (.location (Transformation|GetSocketTransform (Variables|Default|GetWieldedWeapon) "LeftHandPosSocket" "RTS_World")))
  (Variables|Default|SetRightHandPose (.location (Transformation|GetSocketTransform (Variables|Default|GetWieldedWeapon) "RightHandPosSocket" "RTS_World"))))

(event EventInteractwith
  (params (Character :type Character%20Object%20Reference))
  (bind _asbp_parent_unit_class (Utilities|Casting|CastToBP_ParentUnitClass Character))
  (Default|AttackEnemyPawn _asbp_parent_unit_class self))

(fn ConstructionScript)

(fn GetAttackRange
  (return 0.0))

(fn GetIdealRange
  (return 1.5e+02 3e+02))

(fn GetPatrolRoute
  (return (Variables|AI|GetPatrolRoute)))

(fn SetMovementSpeed
  (params (Speed :type E_Movement_Speed%20Enum :default "NewEnumerator0"))
  (bind _output_get (Variables|/Script/Engine.CharacterMovementComponent|SetMaxWalkSpeed (Variables|Character|GetCharacterMovement) (Utilities|Select :Index Speed :NewEnumerator0 0.0 :NewEnumerator1 1e+02 :NewEnumerator2 3e+02 :NewEnumerator3 5e+02)))
  (return _output_get))