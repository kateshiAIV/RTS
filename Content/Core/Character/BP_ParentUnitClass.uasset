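; Base character class for player-commanded units, with cursor highlighting and selection synced between a decal and a HUD icon.
; Handles group moves to randomized nearby points, proximity interaction and a looping move-montage-damage attack.
; When crouched, attacks become backstab takedowns using motion warping and paired montages, with stats deciding kill or survival.
; Moving earns Athletism XP on Tick, and each level-up recalculates walk speed.
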(event OnBeginCursorOver(CapsuleComponent)
  (params (TouchedComponent :type Primitive%20Component%20Object%20Reference))
  (CallFunction|HighlightUnit)
  (Class|Image|SetBrushTintColor (Variables|/Game/Core/Widgets/WidgetSubMenus/WBP_SelectedUnitImage.WBP_SelectedUnitImage_C|GetUnitIcon (Variables|Default|GetWBP_UnitImageRef)) (Utilities|Struct|MakeSlateColor "(R=0.000000,G=1.000000,B=0.070058,A=1.000000)")))

(event OnEndCursorOver(CapsuleComponent)
  (params (TouchedComponent :type Primitive%20Component%20Object%20Reference))
  (bind _wbp_unitimageref (Variables|Default|GetWBP_UnitImageRef))
  (bind _uniticon (Variables|/Game/Core/Widgets/WidgetSubMenus/WBP_SelectedUnitImage.WBP_SelectedUnitImage_C|GetUnitIcon _wbp_unitimageref))
  (CallFunction|UnhighlightUnit)
  (if (Variables|Default|GetUnitIsSelected)
    (Class|Image|SetBrushTintColor _uniticon (Utilities|Struct|MakeSlateColor "(R=0.000000,G=1.000000,B=0.909804,A=1.000000)"))
    (else
      (Class|Image|SetBrushTintColor _uniticon (Utilities|Struct|MakeSlateColor "(R=1.000000,G=1.000000,B=1.000000,A=1.000000)")))))

(event Custom|Attack1
  (params (CurrentAttackTarget :type Actor%20Object%20Reference))
  ;[1 1 1] Attack Logic
  (AI|AIMoveTo self "0, 0, 0" CurrentAttackTarget 2.5e+02 false
    (:OnSuccess
      (AI|SetFocus (AI|GetAIController self) CurrentAttackTarget)
      (Animation|Montage|PlayMontage (Variables|Character|GetMesh) "/Game/Core/Character/Animations/Attack1_Montage.Attack1_Montage"
        (:then
          (Class|AISenseDamage|ReportDamageEvent CurrentAttackTarget self 1e+01 (Transformation|GetActorLocation) "0, 0, 0" "None"))
        (:OnCompleted
          (AI|ClearFocus (AI|GetAIController self) :!label _label)
          (bind _currentattacktarget (Variables|Default|GetCurrentAttackTarget)
            (:then
              (CallFunction|Attack1 _currentattacktarget))
            (:else)))
        (:OnInterrupted
          (goto _label))))))

(event Custom|FocusUnitEvent
  ;[1 1 1] Cast To Controller Focusing Current Unit
  (bind _asbp_top_down_controller (Utilities|Casting|CastToBP_TopDownController (Game|GetPlayerController 0)))
  (Default|FocusUnitEvent _asbp_top_down_controller self))

(event Custom|SetCrouchTRUE
  (Utilities|FlowControl|FlipFlop
    (:A
      (Variables|Crouch|SetisCrouching true))
    (:B
      (Variables|Crouch|SetisCrouching false))))

(event Custom|StealthAttack
  (params (CurrentAttackTarget :type Actor%20Object%20Reference))
  ;[1 1 1] StealthAttack
  (bind _asbp_enemy_base (Utilities|Casting|CastToBP_EnemyBase CurrentAttackTarget))
  (bind _output_get (Variables|Default|SetBP_EnemyBaseRef _asbp_enemy_base))
  (AI|AIMoveTo self "0, 0, 0" _output_get 3e+01 false
    (:OnSuccess
      (if (not (Variables|/Game/Core/CharactersNotPlayable/BP_EnemyBase.BP_EnemyBase_C|GetIsDead _output_get))
        (if (Variables|/Game/Core/CharactersNotPlayable/BP_EnemyBase.BP_EnemyBase_C|GetStealthBackTrigger _output_get)
          (CallFunction|PlayStealthKillAnimation))))))

(event Custom|PlayStealthKillAnimation
  ;[1 1 1] Play Stealth Attack Montage / Calculate Chances
  (CallFunction|MotionWarpingFunc "Target")
  (Utilities|PlayStealthMontages "/Game/Core/Animations/Unarm/AM_Katana_StealthTakedown_Unarm_Attacker01.AM_Katana_StealthTakedown_Unarm_Attacker01" "/Game/Core/Animations/Unarm/AM_Katana_StealthTakedown_Unarm_Victim01.AM_Katana_StealthTakedown_Unarm_Victim01"
    (:VictimSurvived
      (Class|AISenseDamage|ReportDamageEvent (stale Custom|StealthAttack _output_get) self 1e+01 (Transformation|GetActorLocation) "0, 0, 0" "None"))))

(event Custom|Noise
  (Class|Actor|MakeNoise 1.0 self (Transformation|GetActorLocation) 0.0 "None"))

(event EventBeginPlay
  ;[1 1 1] Add Unit Icon to Widget
  (Utilities|FlowControl|Sequence
    (:then_0
      (bind _returnvalue (UserInterface|CreateWidget "/Game/Core/Widgets/WidgetSubMenus/WBP_SelectedUnitImage.WBP_SelectedUnitImage_C"))
      (bind _output_get (Variables|Default|SetWBP_UnitImageRef _returnvalue))
      (Variables|/Game/Core/Widgets/WidgetSubMenus/WBP_SelectedUnitImage.WBP_SelectedUnitImage_C|SetUnitRef _output_get self)
      (Appearance|SetBrushfromTexture (Variables|/Game/Core/Widgets/WidgetSubMenus/WBP_SelectedUnitImage.WBP_SelectedUnitImage_C|GetUnitIcon _returnvalue) (Variables|Default|GetUnitIcon) false)
      (Utilities|FlowControl|Delay 0.2)
      (Class|BPISelection|AddUnittoSelectedUnitsArea(Message) (Game|GetPlayerController 0) (Variables|Default|GetWBP_UnitImageRef)))
    (:then_1
      ;[1 1 1] Set Initial Values
      (StatsSystem|SetValues))))

(event EventStopMovement
  (Components|Movement|StopMovementImmediately (Variables|Character|GetCharacterMovement)))

(event EventSetAttackTarget
  (params (Actor :type Actor%20Object%20Reference))
  ;[1 1 1] Set Attack Target
  (if (Utilities|IsValid Actor)
    (bind _output_get (Variables|Default|SetCurrentAttackTarget Actor))
    (if (not (Variables|Crouch|GetisCrouching))
      (CallFunction|Attack1 _output_get)
      (else
        (CallFunction|StealthAttack _output_get)))))

(event EventSelectUnit
  (bind _wbp_unitimageref (Variables|Default|GetWBP_UnitImageRef))
  ;[1 1 1] Set Decal Visible / Select Unit
  (Variables|Default|SetUnitIsSelected true)
  (Rendering|SetVisibility (Variables|Default|GetSelectionDecal) true false)
  (Class|Image|SetBrushTintColor (Variables|/Game/Core/Widgets/WidgetSubMenus/WBP_SelectedUnitImage.WBP_SelectedUnitImage_C|GetUnitIcon _wbp_unitimageref) (Utilities|Struct|MakeSlateColor "(R=0.000000,G=1.000000,B=0.909804,A=1.000000)"))
  (Variables|/Game/Core/Widgets/WidgetSubMenus/WBP_SelectedUnitImage.WBP_SelectedUnitImage_C|SetSelected _wbp_unitimageref true)
  (Class|BPILimbsStatus|CastLastSelectedUnit(Message) (Game|GetPlayerController 0) self))

(event EventDeselectUnit
  (bind _wbp_unitimageref (Variables|Default|GetWBP_UnitImageRef))
  ;[1 1 1] Set Decal Invisible / Deselect Unit
  (Variables|Default|SetUnitIsSelected false)
  (Rendering|SetVisibility (Variables|Default|GetSelectionDecal) false false)
  (Class|Image|SetBrushTintColor (Variables|/Game/Core/Widgets/WidgetSubMenus/WBP_SelectedUnitImage.WBP_SelectedUnitImage_C|GetUnitIcon _wbp_unitimageref) (Utilities|Struct|MakeSlateColor "(R=1.000000,G=1.000000,B=1.000000,A=1.000000)"))
  (Variables|/Game/Core/Widgets/WidgetSubMenus/WBP_SelectedUnitImage.WBP_SelectedUnitImage_C|SetSelected _wbp_unitimageref false))

(event EventUnitMoveCommand
  (params (Location :type Vector :default "0, 0, 0"))
  (bind _self self)
  (bind _returnvalue (AI|GetAIController _self))
  ;[1 1 1] MoveTo Logic
  (AI|Navigation|StopMovement _returnvalue)
  (Utilities|GroupNPCMovement _returnvalue false Location 1.5e+02))

(event EventUnhighlightUnit
  ;[1 1 1] Unihighlight Ubit From Overlapped Icon
  (Rendering|Components|Decal|SetDecalMaterial (Variables|Default|GetSelectionDecal) "/Game/Core/Materials/Selected_Decal.Selected_Decal")
  (if (not (Variables|Default|GetUnitIsSelected))
    (Rendering|SetVisibility (Variables|Default|GetSelectionDecal) false false)))

(event EventHighlightUnit
  ;[1 1 1] Highlight Unit From Overlapped Icon
  (Rendering|Components|Decal|SetDecalMaterial (Variables|Default|GetSelectionDecal) "/Game/Core/Materials/Highlight_Decal.Highlight_Decal")
  (Rendering|SetVisibility (Variables|Default|GetSelectionDecal) true false))

(event EventSetInteractTarget
  (params (Actor :type Actor%20Object%20Reference))
  ;[1 1 1] Set Interact Target
  (Variables|Default|SetCurrentInteractTarget Actor))

(event EventTick
  (params (DeltaSeconds :type Float%20%28single-precision%29))
  (Utilities|FlowControl|Sequence
    (:then_0
      ;[1 1 1] Interact Logic
      (bind _currentinteracttarget (Variables|Default|GetCurrentInteractTarget)
        (:then
          (if (<= (Transformation|GetDistanceTo _currentinteracttarget self) (Variables|Default|GetInteractionRadius))
            (Class|BPIInteraction|Interactwith(Message) (Variables|Default|GetCurrentInteractTarget) self)
            (Variables|Default|SetCurrentInteractTarget 0)
            (Components|Movement|StopMovementImmediately (Variables|Character|GetCharacterMovement))))
        (:else)))
    (:then_2
      ;[1 1 1] Update Stats Logic
      (StatsSystem|UpdateStats))))

(fn ConstructionScript)

(fn SetValues
  (Init|SetSpeed))

(fn SetSpeed
  (Variables|/Script/Engine.CharacterMovementComponent|SetMaxWalkSpeed (Variables|Character|GetCharacterMovement) (+ (* 7e+02 (/ (.Value (Utilities|Map|Find (Variables|/Game/Core/Components/BPC_Stats.BPC_Stats_C|GetStats (Variables|Default|GetBPC_Stats)) "Athletism")) 1e+02)) 5e+02)))

(fn UpdateStats
  ;[1 1 1] Check if is Moving
  (if (>= (Math|Vector|VectorLength (Variables|/Script/Engine.MovementComponent|GetVelocity (Variables|Character|GetCharacterMovement))) 1e+01)
    ;[1 1 1] Add XP to Athletism
    (Utilities|Map|Add (Variables|/Game/Core/Components/BPC_Stats.BPC_Stats_C|GetCurrentXP (Variables|Default|GetBPC_Stats)) "Athletism" (+ (.Value (Utilities|Map|Find (Variables|/Game/Core/Components/BPC_Stats.BPC_Stats_C|GetCurrentXP (Variables|Default|GetBPC_Stats)) "Athletism")) (* (LocalVariables|GetXP) (Class|GameplayStatics|GetGlobalTimeDilation))))
    ;[1 1 1] Check if Current XP is Greater That Max XP
    (if (>= (.Value (Utilities|Map|Find (Variables|/Game/Core/Components/BPC_Stats.BPC_Stats_C|GetCurrentXP (Variables|Default|GetBPC_Stats)) "Athletism")) (.Value (Utilities|Map|Find (Variables|/Game/Core/Components/BPC_Stats.BPC_Stats_C|GetMaxXP (Variables|Default|GetBPC_Stats)) "Athletism")))
      ;[1 1 1] 0 Current XP, Multiply MAX XP
      (Utilities|Map|Add (Variables|/Game/Core/Components/BPC_Stats.BPC_Stats_C|GetCurrentXP (Variables|Default|GetBPC_Stats)) "Athletism" (* (.Value (Utilities|Map|Find (Variables|/Game/Core/Components/BPC_Stats.BPC_Stats_C|GetCurrentXP (Variables|Default|GetBPC_Stats)) "Athletism")) 0.0))
      (Utilities|Map|Add (Variables|/Game/Core/Components/BPC_Stats.BPC_Stats_C|GetMaxXP (Variables|Default|GetBPC_Stats)) "Athletism" (* (.Value (Utilities|Map|Find (Variables|/Game/Core/Components/BPC_Stats.BPC_Stats_C|GetMaxXP (Variables|Default|GetBPC_Stats)) "Athletism")) 1.5))
      ;[1 1 1] Add level to Athetism
      (Utilities|Map|Add (Variables|/Game/Core/Components/BPC_Stats.BPC_Stats_C|GetStats (Variables|Default|GetBPC_Stats)) "Athletism" (+ (.Value (Utilities|Map|Find (Variables|/Game/Core/Components/BPC_Stats.BPC_Stats_C|GetStats (Variables|Default|GetBPC_Stats)) "Athletism")) 1.0))
      (Init|SetSpeed))))

(fn MotionWarpingFunc
  (params (WarpTargetName :type Name))
  (bind _asbp_enemy_base (Utilities|Casting|CastToBP_EnemyBase (Variables|Default|GetCurrentPotentialStealthTarget)))
  (if (Variables|/Game/Core/CharactersNotPlayable/BP_EnemyBase.BP_EnemyBase_C|GetStealthBackTrigger _asbp_enemy_base)
    (Class|MotionWarpingComponent|AddorUpdateWarpTargetfromTransform (Variables|Default|GetBPC_MotionWarping) WarpTargetName (Transformation|GetWorldTransform (Variables|/Game/Core/CharactersNotPlayable/BP_EnemyBase.BP_EnemyBase_C|GetStealthKillPosition _asbp_enemy_base)))))

(fn GetAttackRange
  (return 1.5e+02))

(fn GrabSelectedUnits
  (return 0))