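; Actor component that tracks health for six body parts (head, torso, hands, legs) and handles healing, with no damage logic present.
; While CanHeal is set, Tick regenerates each part below its max by HealthMultiplier per frame, unscaled by delta time and clamped to a fixed 100.
; Heal adds an amount to one chosen part unless dead, clamps to that part's max, and returns the new health and part.
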(event EventBeginPlay)

(event EventTick
  (params (DeltaSeconds :type Float%20%28single-precision%29))
  (CallFunction|UpdateHealthStats))

(fn UpdateHealthStats
  (if (Variables|Default|GetCanHeal?)
    (Utilities|FlowControl|Sequence
      (:then_0
        (if (< (Variables|LeftLeg|GetLLCurrentHealth) (Variables|LeftLeg|GetLLMaxHealth))
          (Variables|LeftLeg|SetLLCurrentHealth (Math|Float|Clamp(Float) (+ (Variables|LeftLeg|GetLLCurrentHealth) (Variables|Default|GetHealthMultiplier)) 0.0 1e+02))))
      (:then_1
        (if (< (Variables|RightLeg|GetRLCurrentHealth) (Variables|RightLeg|GetRLMaxHealth))
          (Variables|RightLeg|SetRLCurrentHealth (Math|Float|Clamp(Float) (+ (Variables|RightLeg|GetRLCurrentHealth) (Variables|Default|GetHealthMultiplier)) 0.0 1e+02))))
      (:then_2
        (if (< (Variables|LeftHand|GetLHCurrentHealth) (Variables|LeftHand|GetLHMaxHealth))
          (Variables|LeftHand|SetLHCurrentHealth (Math|Float|Clamp(Float) (+ (Variables|LeftHand|GetLHCurrentHealth) (Variables|Default|GetHealthMultiplier)) 0.0 1e+02))))
      (:then_3
        (if (< (Variables|RightHand|GetRHCurrentHealth) (Variables|RightHand|GetRHMaxHealth))
          (Variables|RightHand|SetRHCurrentHealth (Math|Float|Clamp(Float) (+ (Variables|RightHand|GetRHCurrentHealth) (Variables|Default|GetHealthMultiplier)) 0.0 1e+02))))
      (:then_4
        (if (< (Variables|Torso|GetTorsoCurrentHealth) (Variables|Torso|GetTorsoMaxHealth))
          (Variables|Torso|SetTorsoCurrentHealth (Math|Float|Clamp(Float) (+ (Variables|Torso|GetTorsoCurrentHealth) (Variables|Default|GetHealthMultiplier)) 0.0 1e+02))))
      (:then_5
        (if (< (Variables|Head|GetHeadCurrentHealth) (Variables|Head|GetHeadMaxHealth))
          (Variables|Head|SetHeadCurrentHealth (Math|Float|Clamp(Float) (+ (Variables|Head|GetHeadCurrentHealth) (Variables|Default|GetHealthMultiplier)) 0.0 1e+02)))))))

(fn Heal
  (params (Amount :type Float%20%28double-precision%29) (BodyPart :type E_BodyParts%20Enum :default "NewEnumerator0"))
  (if (not (Variables|Default|GetIsDead))
    (switch Utilities|FlowControl|Switch|SwitchonE_BodyParts BodyPart
      (:NewEnumerator0
        (bind _output_get (Variables|Head|SetHeadCurrentHealth (Math|Float|Clamp(Float) (+ Amount (Variables|Head|GetHeadCurrentHealth)) 0.0 (Variables|Head|GetHeadMaxHealth))))
        (return _output_get BodyPart))
      (:NewEnumerator1
        (bind _output_get_2 (Variables|Torso|SetTorsoCurrentHealth (Math|Float|Clamp(Float) (+ (Variables|Torso|GetTorsoCurrentHealth) Amount) 0.0 (Variables|Torso|GetTorsoMaxHealth))))
        (return _output_get_2 BodyPart))
      (:NewEnumerator2
        (bind _output_get_3 (Variables|RightHand|SetRHCurrentHealth (Math|Float|Clamp(Float) (+ (Variables|RightHand|GetRHCurrentHealth) Amount) 0.0 (Variables|RightHand|GetRHMaxHealth))))
        (return _output_get_3 BodyPart))
      (:NewEnumerator3
        (bind _output_get_4 (Variables|LeftHand|SetLHCurrentHealth (Math|Float|Clamp(Float) (+ (Variables|LeftHand|GetLHCurrentHealth) Amount) 0.0 (Variables|LeftHand|GetLHMaxHealth))))
        (return _output_get_4 BodyPart))
      (:NewEnumerator4
        (bind _output_get_5 (Variables|RightLeg|SetRLCurrentHealth (Math|Float|Clamp(Float) (+ (Variables|RightLeg|GetRLCurrentHealth) Amount) 0.0 (Variables|RightLeg|GetRLMaxHealth))))
        (return _output_get_5 BodyPart))
      (:NewEnumerator5
        (bind _output_get_6 (Variables|LeftLeg|SetLLCurrentHealth (Math|Float|Clamp(Float) (+ (Variables|LeftLeg|GetLLCurrentHealth) Amount) 0.0 (Variables|LeftLeg|GetLLMaxHealth))))
        (return _output_get_6 BodyPart)))))