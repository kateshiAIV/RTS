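; Health component that tracks separate health pools for head, torso, both legs and both hands, and regenerates them over time.
; Every Tick calls UpdateHealthStats, which, while CanHeal is true, adds HealthMultiplier to each part below its max.
; The increment is not scaled by delta time, so healing speed depends on frame rate.
; Results clamp to a fixed 0–100 range rather than each part's max.
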(event EventBeginPlay)

(event EventTick
  (params (DeltaSeconds :type Float%20%28single-precision%29))
  (CallFunction|UpdateHealthStats))

(fn UpdateHealthStats
  (if (Variables|Default|GetCanHeal?)
    (Utilities|FlowControl|Sequence
      (:then_0
        (if (< (Variables|LeftLeg|GetLLCurrentHealth) (Variables|LeftLeg|GetLLMaxHealth))
          (Variables|LeftLeg|SetLLCurrentHealth (Math|Float|Clamp(Float) (+ (Variables|LeftLeg|GetLLCurrentHealth) (Variables|Default|GetHealthMultiplier)) 0.0 1e+02))))
      (:then_1
        (if (< (Variables|RightLeg|GetRLCurrentHealth) (Variables|RightLeg|GetRLMaxHealth))
          (Variables|RightLeg|SetRLCurrentHealth (Math|Float|Clamp(Float) (+ (Variables|RightLeg|GetRLCurrentHealth) (Variables|Default|GetHealthMultiplier)) 0.0 1e+02))))
      (:then_2
        (if (< (Variables|LeftHand|GetLHCurrentHealth) (Variables|LeftHand|GetLHMaxHealth))
          (Variables|LeftHand|SetLHCurrentHealth (Math|Float|Clamp(Float) (+ (Variables|LeftHand|GetLHCurrentHealth) (Variables|Default|GetHealthMultiplier)) 0.0 1e+02))))
      (:then_3
        (if (< (Variables|RightHand|GetRHCurrentHealth) (Variables|RightHand|GetRHMaxHealth))
          (Variables|RightHand|SetRHCurrentHealth (Math|Float|Clamp(Float) (+ (Variables|RightHand|GetRHCurrentHealth) (Variables|Default|GetHealthMultiplier)) 0.0 1e+02))))
      (:then_4
        (if (< (Variables|Torso|GetTorsoCurrentHealth) (Variables|Torso|GetTorsoMaxHealth))
          (Variables|Torso|SetTorsoCurrentHealth (Math|Float|Clamp(Float) (+ (Variables|Torso|GetTorsoCurrentHealth) (Variables|Default|GetHealthMultiplier)) 0.0 1e+02))))
      (:then_5
        (if (< (Variables|Head|GetHeadCurrentHealth) (Variables|Head|GetHeadMaxHealth))
          (Variables|Head|SetHeadCurrentHealth (Math|Float|Clamp(Float) (+ (Variables|Head|GetHeadCurrentHealth) (Variables|Default|GetHealthMultiplier)) 0.0 1e+02)))))))