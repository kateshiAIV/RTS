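; BP_SunRotation is an actor that rotates a referenced sun actor to match the game time of day.
; Each Tick it sets SunRef's rotation from CalculateSunRotation, which maps GameTime on a 24-hour cycle to a full pitch revolution with fixed yaw and roll.
; GameTime changes only through the SetGameTime event, and the actor destroys itself on BeginPlay when SunRef is invalid.
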(event EventBeginPlay
  (Variables|Default|GetSunRef
    (:then)
    (:else
      (Actor|DestroyActor))))

(event Collision|EventActorBeginOverlap
  (params (OtherActor :type Actor%20Object%20Reference)))

(event EventTick
  (params (DeltaSeconds :type Float%20%28single-precision%29))
  (bind _sunref (Variables|Default|GetSunRef)
    (:then
      (Transformation|SetActorRotation _sunref (CallFunction|CalculateSunRotation)))
    (:else)))

(event EventSetGameTime
  (params (GameTime :type Float%20%28double-precision%29))
  (Variables|Default|SetGameTime GameTime))

(fn ConstructionScript)

(fn CalculateSunRotation
  (return (Math|Rotator|MakeRotator 25.0 (+ (* (/ (Math|Float|%(Float) (Variables|Default|GetGameTime) 24.0) 24.0) 3.6e+02) 9e+01) 25.0)))