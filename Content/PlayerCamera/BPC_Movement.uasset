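; BPC_Movement is a camera movement component that drives its owning BP_Camera with axis movement, edge scrolling, yaw panning, zoom and resets.
; Movement functions apply swept local offsets scaled by speed settings, with adjustable, clamped base speed.
; Zoom calls set a normalized target that Tick lerps toward and passes to SetArmLength.
; Edge scrolling tests viewport-relative mouse position, using a diagonal speed computed once at init; its bottom-edge-only branch is unwired.
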(event Custom|InitComponent
  (bind _asbp_camera (Utilities|Casting|CastToBP_Camera (Components|GetOwner)))
  (Variables|Default|SetCameraRef _asbp_camera)
  (CallFunction|DetermineEdgeScrollSpeed))

(event EventBeginPlay)

(event EventTick
  (params (DeltaSeconds :type Float%20%28single-precision%29))
  (CallFunction|ZoomEvents))

(fn BasicMovementControls
  (params (AxisX :type Float%20%28double-precision%29) (AxisY :type Float%20%28double-precision%29))
  (LocalVariables|SetXLocal AxisX)
  (LocalVariables|SetYLocal AxisY)
  (if (not (Variables|Default|GetbDisableCamera))
    (if (and (!= (LocalVariables|GetYLocal) 0.0) (!= (LocalVariables|GetXLocal) 0.0))
      (Transformation|AddActorLocalOffset (Variables|Default|GetCameraRef) (+ (Math|Vector|MakeVector (* (LocalVariables|GetXLocal) (Variables|Default|GetDefaultMovementSpeed) (Variables|Default|GetMovementSpeedModifier)) 0.0 0.0) (Math|Vector|MakeVector 0.0 (* (LocalVariables|GetYLocal) (Variables|Default|GetDefaultMovementSpeed) (Variables|Default|GetMovementSpeedModifier)) 0.0)) true false)
      (elif (!= (LocalVariables|GetXLocal) 0.0)
        (Transformation|AddActorLocalOffset (Variables|Default|GetCameraRef) (Math|Vector|MakeVector (* (LocalVariables|GetXLocal) (Variables|Default|GetDefaultMovementSpeed) (Variables|Default|GetMovementSpeedModifier)) 0.0 0.0) true false)
        (elif (!= (LocalVariables|GetYLocal) 0.0)
          (Transformation|AddActorLocalOffset (Variables|Default|GetCameraRef) (Math|Vector|MakeVector 0.0 (* (LocalVariables|GetYLocal) (Variables|Default|GetDefaultMovementSpeed) (Variables|Default|GetMovementSpeedModifier)) 0.0) true false))))))

(fn Zoomin
  (bind _output_get (Variables|Default|SetDeltaZoomAmount (+ (Variables|Default|GetDeltaZoomAmount) 0.1)))
  (if (> _output_get 1.0)
    (Variables|Default|SetDeltaZoomAmount 1.0))
  (return))

(fn ZoomOut
  (bind _output_get (Variables|Default|SetDeltaZoomAmount (- (Variables|Default|GetDeltaZoomAmount) 0.1)))
  (if (< _output_get 0.0)
    (Variables|Default|SetDeltaZoomAmount 0.0))
  (return))

(fn ResetZoom
  (Variables|Default|SetDeltaZoomAmount 0.5)
  (return))

(fn ZoomEvents
  (bind _output_get (Variables|Default|SetZoomAmount (Math|Float|Lerp (Variables|Default|GetZoomAmount) (Variables|Default|GetDeltaZoomAmount) 0.1)))
  (Default|SetArmLength (Variables|Default|GetCameraRef) _output_get)
  (return))

(fn PanCamera
  (params (RotationAmount :type Float%20%28double-precision%29))
  (bind _cameraref (Variables|Default|GetCameraRef))
  (Transformation|SetActorRotation _cameraref (Math|Rotator|CombineRotators (Math|Rotator|MakeRotator 0.0 0.0 RotationAmount) (Transformation|GetActorRotation _cameraref)))
  (return))

(fn ResetPan
  (Transformation|SetActorRotation (Variables|Default|GetCameraRef))
  (return))

(fn ResetCamera
  (CallFunction|ResetZoom)
  (CallFunction|ResetPan)
  (return))

(fn SetDisableEdgeScroll
  (params (bDisableEdgeScroll :type Boolean))
  (Variables|Default|SetbDisableEdgeScroll bDisableEdgeScroll)
  (return))

(fn DetermineEdgeScrollSpeed
  (Variables|Default|SetCornerEgdeScrollSpeed (* (Variables|Default|GetDefaultMovementSpeed) (Math|Float|Sqrt 0.5))))

(fn EdgeScroll
  (bind _returnvalue (Game|GetPlayerController 0))
  (bind _returnvalue_2 (Viewport|GetViewportSize))
  (bind _movementspeedmodifier (Variables|Default|GetMovementSpeedModifier))
  (bind _movementspeedmodifier_2 (Variables|Default|GetMovementSpeedModifier))
  (bind _movementspeedmodifier_3 (Variables|Default|GetMovementSpeedModifier))
  (bind _movementspeedmodifier_4 (Variables|Default|GetMovementSpeedModifier))
  (bind (_locationx _locationy) (Game|Player|GetMousePosition _returnvalue))
  (bind _returnvalue_3 (/ _locationx (.x _returnvalue_2)))
  (bind _returnvalue_4 (/ _locationy (.y _returnvalue_2)))
  (bind _returnvalue_5 (>= _returnvalue_4 0.95))
  (bind _returnvalue_6 (<= _returnvalue_4 0.05))
  (bind _returnvalue_7 (>= _returnvalue_3 0.95))
  (bind _returnvalue_8 (<= _returnvalue_3 0.05))
  (if (not (Variables|Default|GetbDisableCamera))
    (if (and _returnvalue_7 _returnvalue_6)
      (CallFunction|SetCameraDisabled false)
      (LocalVariables|SetDeltaSpeedXLocal (* (Variables|Default|GetCornerEgdeScrollSpeed) _movementspeedmodifier_4))
      (LocalVariables|SetDeltaSpeedYLocal _movementspeedmodifier_4)
      (Transformation|AddActorLocalOffset (Variables|Default|GetCameraRef) (Math|Vector|MakeVector (LocalVariables|GetDeltaSpeedYLocal) (LocalVariables|GetDeltaSpeedXLocal) 0.0) true false :!label _label)
      (return)
      (elif (and _returnvalue_7 _returnvalue_5)
        (CallFunction|SetCameraDisabled false)
        (LocalVariables|SetDeltaSpeedXLocal (* (Variables|Default|GetCornerEgdeScrollSpeed) _movementspeedmodifier_3))
        (LocalVariables|SetDeltaSpeedYLocal (* _movementspeedmodifier_3 -1.0))
        (goto _label)
        (elif (and _returnvalue_8 _returnvalue_6)
          (CallFunction|SetCameraDisabled false)
          (LocalVariables|SetDeltaSpeedXLocal (* (Variables|Default|GetCornerEgdeScrollSpeed) _movementspeedmodifier -1.0))
          (LocalVariables|SetDeltaSpeedYLocal _movementspeedmodifier)
          (goto _label)
          (elif (and _returnvalue_8 _returnvalue_5)
            (CallFunction|SetCameraDisabled false)
            (LocalVariables|SetDeltaSpeedXLocal (* (Variables|Default|GetCornerEgdeScrollSpeed) _movementspeedmodifier_2 -1.0))
            (LocalVariables|SetDeltaSpeedYLocal (* _movementspeedmodifier_2 -1.0))
            (goto _label)
            (elif _returnvalue_7
              (CallFunction|SetCameraDisabled false)
              (LocalVariables|SetDeltaSpeedXLocal (* (Variables|Default|GetCornerEgdeScrollSpeed) (Variables|Default|GetMovementSpeedModifier)))
              (LocalVariables|SetDeltaSpeedYLocal 0.0)
              (goto _label)
              (elif _returnvalue_8
                (CallFunction|SetCameraDisabled false)
                (LocalVariables|SetDeltaSpeedXLocal (* (Variables|Default|GetCornerEgdeScrollSpeed) (Variables|Default|GetMovementSpeedModifier) -1.0))
                (LocalVariables|SetDeltaSpeedYLocal 0.0)
                (goto _label)
                (elif (not _returnvalue_5)
                  (if _returnvalue_6
                    (CallFunction|SetCameraDisabled false)
                    (LocalVariables|SetDeltaSpeedXLocal 0.0)
                    (LocalVariables|SetDeltaSpeedYLocal (* (Variables|Default|GetCornerEgdeScrollSpeed) (Variables|Default|GetMovementSpeedModifier)))
                    (goto _label)
                    (else
                      (CallFunction|SetCameraDisabled false)
                      (LocalVariables|SetDeltaSpeedXLocal 0.0)
                      (LocalVariables|SetDeltaSpeedYLocal 0.0)
                      (goto _label))))))))))))

(fn SetCameraDisabled
  (params (bDisableCamera :type Boolean))
  (Variables|Default|SetbDisableCamera bDisableCamera)
  (return))

(fn IncreaseCameraSpeed
  (bind _output_get (Variables|Default|SetDefaultMovementSpeed (Math|Float|Clamp(Float) (+ (Variables|Default|GetDefaultMovementSpeed) (Variables|Default|GetMovementSpeedModifier)) 0.0 5e+01)))
  (Development|PrintString (Utilities|String|ToString(Float) _output_get)))

(fn DecreaseCameraSpeed
  (bind _output_get (Variables|Default|SetDefaultMovementSpeed (Math|Float|Clamp(Float) (- (Variables|Default|GetDefaultMovementSpeed) (Variables|Default|GetMovementSpeedModifier)) 0.0 5e+01)))
  (Development|PrintString (Utilities|String|ToString(Float) _output_get)))